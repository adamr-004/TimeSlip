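; TSTut_BP is a one-shot trigger volume that shows a tutorial message when BP_Timekeeper overlaps its box.
; On overlap it makes the Okay, TutorialText and blurred background widgets on that actor's HUD visible.
; It then pauses the game, switches input to UI only with the mouse cursor shown, and destroys itself.
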(event OnComponentBeginOverlap(Box)
  (params (OverlappedComponent :type Primitive%20Component%20Object%20Reference) (OtherActor :type Actor%20Object%20Reference) (OtherComp :type Primitive%20Component%20Object%20Reference) (OtherBodyIndex :type Integer) (bFromSweep :type Boolean) (SweepResult :type Hit%20Result%20Structure%20%28by%20ref%29))
  (bind _returnvalue (Game|GetPlayerController 0))
  (bind _asbp_timekeeper (Utilities|Casting|CastToBP_Timekeeper OtherActor))
  (Widget|SetVisibility (Variables|/Game/HUDSnUIS/HUD_widget.HUD_widget_C|Getokay (Variables|/Game/FirstPerson/Blueprints/BP_Timekeeper.BP_Timekeeper_C|GetHUD _asbp_timekeeper)) "Visible")
  (Game|SetGamePaused true)
  (Input|SetInputModeUIOnly _returnvalue 0 "DoNotLock" false)
  (Variables|/Script/Engine.PlayerController|SetbShowMouseCursor _returnvalue true)
  (Actor|DestroyActor))

(fn ConstructionScript)